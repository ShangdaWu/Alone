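; Monster actor that fills in its identity, look and stats at random when the player controller signals a monster birth.
; On BeginPlay it binds to the EDBornMonster dispatcher on Alone_PlayerController.
; Each broadcast picks one of three Monster DataTable rows by random number, setting the name text and four plane materials.
; The row also feeds current and target blood to the UI_MonsterPanel widget and stores the movement speed.
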(event `self.ReceiveBeginPlay`
  (bind _asalone_player_controller (cast `/Game/Mode/Alone_PlayerController` (`GameplayStatics.GetPlayerController` 0)))
  ;[1 1 1] 生成怪物基础数据
  (add `/Game/Mode/Alone_PlayerController.ED_BornMonster` _asalone_player_controller (delegate `CustomEvent_BronMonster`)))

(event `CustomEvent_BronMonster`
  ;[1 1 1] 生成怪物基础数据
  (bind _output_get (set `self.MonsterName` (`KismetStringLibrary.Conv_StringToName` (`KismetStringLibrary.Conv_IntToString` (`KismetMathLibrary.RandomIntegerInRange` 1 3)))))
  (bind _returnvalue (`|GetDataTableRow` "/Game/Data/Monster.Monster" _output_get)
    (:`then`
      (bind (_name _level _blood_current _blood_target _armor _resist _crit _hit_dice _dodge _block _parry _defense _block_2 _parry_2 _speed _attack_times _attack_base _attack_dice _skill _treasure _run _type _type_a _type_b _type_c _type_d) (break `/Game/Data/Monster_Data` _returnvalue))
      (`TextRenderComponent.K2_SetText` (`self.Monster_Name`) _name)
      (`PrimitiveComponent.SetMaterial` (`self.Plane_A`) 0 _type_a)
      (`PrimitiveComponent.SetMaterial` (`self.Plane_B`) 0 _type_b)
      (`PrimitiveComponent.SetMaterial` (`self.Plane_C`) 0 _type_c)
      (`PrimitiveComponent.SetMaterial` (`self.Plane_D`) 0 _type_d)
      (bind _asui_monster_panel (cast `/Game/UMG/UI_MonsterPanel` (`WidgetComponent.GetUserWidgetObject` (`self.Monster_Panel`))))
      (set `/Game/UMG/UI_MonsterPanel.Monster_BloodCurrent` _blood_current _asui_monster_panel)
      (set `/Game/UMG/UI_MonsterPanel.Monster_BloodTarget` _blood_target _asui_monster_panel)
      (set `self.MonsterSpeed` _speed))))

(fn `UserConstructionScript`
  (`parent.UserConstructionScript`))