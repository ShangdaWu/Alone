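; BP_Monster_B is one of three selectable monster slots (A, B, C) that the player can pick as an attack target.
; On the player controller's born-monster event, it loads a random Monster data table row into its name, four plane materials, health panel and speed.
; Clicking it plays a sound, marks it selected and records its ID on the controller.
; It deselects A and C through fixed GetAllActorsOfClass indices, relying on array order.
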(event `self.ReceiveBeginPlay`
  (bind _asalone_player_controller (cast `/Game/Mode/Alone_PlayerController` (`GameplayStatics.GetPlayerController` 0)))
  ;[1 1 1] 生成怪物基础数据
  (add `/Game/Mode/Alone_PlayerController.ED_BornMonster` _asalone_player_controller (delegate `CustomEvent_BronMonster`)))

(event `CustomEvent_BronMonster`
  ;[1 1 1] 生成怪物基础数据
  (bind _output_get (set `self.MonsterName` (`KismetStringLibrary.Conv_StringToName` (`KismetStringLibrary.Conv_IntToString` (`KismetMathLibrary.RandomIntegerInRange` 1 3)))))
  (bind _returnvalue (`|GetDataTableRow` "/Game/Data/Monster.Monster" _output_get)
    (:`then`
      (bind (_name _level _blood_current _blood_target _armor _resist _crit _hit_dice _dodge _block _parry _speed _attack_times _attack_base _attack_dice _skill _treasure _run _type _type_a _type_b _type_c _type_d) (break `/Game/Data/Monster_Data` _returnvalue))
      (`TextRenderComponent.K2_SetText` (`self.Monster_Name`) _name)
      (`PrimitiveComponent.SetMaterial` (`self.Plane_A`) 0 _type_a)
      (`PrimitiveComponent.SetMaterial` (`self.Plane_B`) 0 _type_b)
      (`PrimitiveComponent.SetMaterial` (`self.Plane_C`) 0 _type_c)
      (`PrimitiveComponent.SetMaterial` (`self.Plane_D`) 0 _type_d)
      (bind _asui_monster_panel (cast `/Game/UMG/UI_MonsterPanel` (`WidgetComponent.GetUserWidgetObject` (`self.Monster_Panel`))))
      (set `/Game/UMG/UI_MonsterPanel.Monster_BloodCurrent` _blood_current _asui_monster_panel)
      (set `/Game/UMG/UI_MonsterPanel.Monster_BloodTarget` _blood_target _asui_monster_panel)
      (set `self.MonsterSpeed` _speed))))

(event `self.Clicked_Box.OnClicked`
  (params (TouchedComponent :type "PrimitiveComponent Object Reference") (ButtonPressed :type "Key Structure"))
  (`GameplayStatics.PlaySound2D` "/Game/Sound/Select_Monster.Select_Monster" 1.0 1.0 0.0 null null)
  (set `self.Select_Monster` true)
  (bind _outactors (`GameplayStatics.GetAllActorsOfClass` "/Game/Monster/BP_BaseMonster.BP_BaseMonster_C"))
  (bind _asbp_monster_a (cast `/Game/Monster/BP_Monster_A` (`|GetArrayItem` _outactors)))
  (bind _asbp_monster_c (cast `/Game/Monster/BP_Monster_C` (`|GetArrayItem` _outactors 2)))
  (set `/Game/Monster/BP_BaseMonster.Select_Monster` false _asbp_monster_a)
  (set `/Game/Monster/BP_BaseMonster.Select_Monster` false _asbp_monster_c)
  (bind _asalone_player_controller (cast `/Game/Mode/Alone_PlayerController` (`GameplayStatics.GetPlayerController` 0)))
  (set `/Game/Mode/Alone_PlayerController.PlayerSelect_AttackMonster_ID` 1 _asalone_player_controller)
  (`KismetSystemLibrary.PrintString` "我是B"))

(fn `UserConstructionScript`
  (`parent.UserConstructionScript`))