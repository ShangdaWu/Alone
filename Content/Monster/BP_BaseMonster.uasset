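; BP_BaseMonster is a monster Blueprint that displays a spinning selection indicator when the monster is selected.
; Each Tick it checks that Alone_PlayerController's MonsterNumber has reached a threshold and that its own SelectMonster flag is set.
; When both hold, it shows TargetBox and plays a timeline that drives SelectBox's world yaw.
; Otherwise it hides TargetBox and stops the timeline.
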(event `self.ReceiveTick`
  (params (DeltaSeconds :type "Float (single-precision)"))
  (bind _target_box (`self.Target_Box`))
  (bind _asalone_player_controller (cast `/Game/Mode/Alone_PlayerController` (`GameplayStatics.GetPlayerController` 0)))
  (if (>= (`/Game/Mode/Alone_PlayerController.Monster_Number` _asalone_player_controller) 70)
    (if (`self.Select_Monster`)
      (`SceneComponent.SetVisibility` _target_box true false)
      (bind (_direction _y) (`Timeline|Timeline_SelectMonster` :!label _label)
        (:`Update`
          (`SceneComponent.K2_SetWorldRotation` (`self.Select_Box`) (`KismetMathLibrary.MakeRotator` 0.0 0.0 _y) true false)))
      (else
        (`SceneComponent.SetVisibility` _target_box false false :!label _label_2)
        (goto _label :!via `Stop`)))
    (else
      (goto _label_2))))

(fn `UserConstructionScript`)